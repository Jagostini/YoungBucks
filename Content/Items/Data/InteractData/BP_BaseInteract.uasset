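; BP_BaseInteract is a base interactable actor with an item mesh and a sphere trigger.
; When a BP_SurvivalCharacter enters or leaves the trigger, the actor registers or unregisters itself with that character as an interactable.
; The construction script applies configurable mesh scale and trigger radius.
; SetOutline toggles the mesh's Render Custom Depth flag for outline highlighting.
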(event `self.TriggerInteract.OnComponentBeginOverlap`
  (params (OverlappedComponent :type "PrimitiveComponent Object Reference") (OtherActor :type "Actor Object Reference") (OtherComp :type "PrimitiveComponent Object Reference") (OtherBodyIndex :type Integer) (bFromSweep :type Boolean) (SweepResult :type "HitResult Structure (by ref)"))
  (bind _asbp_survival_character (cast `/Game/Character/ThirdPersonBP/Blueprints/BP_SurvivalCharacter` OtherActor))
  (message `/Game/Items/Data/InteractData/BPI_Interact.RegisterInteractable` _asbp_survival_character self))

(event `self.TriggerInteract.OnComponentEndOverlap`
  (params (OverlappedComponent :type "PrimitiveComponent Object Reference") (OtherActor :type "Actor Object Reference") (OtherComp :type "PrimitiveComponent Object Reference") (OtherBodyIndex :type Integer))
  (bind _asbp_survival_character (cast `/Game/Character/ThirdPersonBP/Blueprints/BP_SurvivalCharacter` OtherActor))
  (message `/Game/Items/Data/InteractData/BPI_Interact.UnregisterInteractable` _asbp_survival_character self))

(fn `SetOutline`
  (params (`OutLight?` :type Boolean))
  (`PrimitiveComponent.SetRenderCustomDepth` (`self.SM_Item`) `OutLight?`))

(fn `UserConstructionScript`
  (`SceneComponent.SetWorldScale3D` (`self.SM_Item`) (`self.MeshScale`))
  (`SphereComponent.SetSphereRadius` (`self.TriggerInteract`) (`self.TriggerSize`) true))