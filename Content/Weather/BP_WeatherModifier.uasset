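; BP_WeatherModifier is a placeable trigger volume that changes the temperature a survival character experiences inside its area.
; On overlap begin it calls ApplyTempModifier on the BP_SurvivalCharacter, passing an optional world temperature override and an additive modifier.
; On overlap end it clears the override and applies the negated modifier to undo the offset.
; The construction script sizes the AreaZone box from the TriggerSize variable.
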(event `self.AreaZone.OnComponentBeginOverlap`
  (params (OverlappedComponent :type "PrimitiveComponent Object Reference") (OtherActor :type "Actor Object Reference") (OtherComp :type "PrimitiveComponent Object Reference") (OtherBodyIndex :type Integer) (bFromSweep :type Boolean) (SweepResult :type "HitResult Structure (by ref)"))
  (bind _asbp_survival_character (cast `/Game/Character/ThirdPersonBP/Blueprints/BP_SurvivalCharacter` OtherActor))
  (`/Game/Character/ThirdPersonBP/Blueprints/BP_SurvivalCharacter.ApplyTempModifier` _asbp_survival_character (`self.OverrideLocalWorldTemp`) (`self.NewWorldTemp`) (`self.AreaTempModifier`)))

(event `self.AreaZone.OnComponentEndOverlap`
  (params (OverlappedComponent :type "PrimitiveComponent Object Reference") (OtherActor :type "Actor Object Reference") (OtherComp :type "PrimitiveComponent Object Reference") (OtherBodyIndex :type Integer))
  (bind _asbp_survival_character (cast `/Game/Character/ThirdPersonBP/Blueprints/BP_SurvivalCharacter` OtherActor))
  (`/Game/Character/ThirdPersonBP/Blueprints/BP_SurvivalCharacter.ApplyTempModifier` _asbp_survival_character false 0.0 (* (`self.AreaTempModifier`) -1.0)))

(fn `UserConstructionScript`
  (`BoxComponent.SetBoxExtent` (`self.AreaZone`) (`self.TriggerSize`) true))